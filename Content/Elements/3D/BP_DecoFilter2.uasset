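; BP_DecoFilter2 is a decorative static mesh actor that changes its material to match the current color filter in the VR game mode.
; On BeginPlay it applies its configured mesh, caches the VRGameMode and binds to its filter-changed event.
; Each change sets material slot 0 to the test material for None, Red, Green or Blue, with no initial update at startup.
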(event `self.ReceiveBeginPlay`
  (`StaticMeshComponent.SetStaticMesh` (`self.StaticMesh`) (`self.StaticMeshToSet`))
  (bind _asvrgame_mode (cast `/Game/VRTemplate/Blueprints/VRGameMode` (`GameplayStatics.GetGameMode`)))
  (bind _output_get (set `self.VRGameModeRef` _asvrgame_mode))
  (add `/Game/VRTemplate/Blueprints/VRGameMode.FilterChanged` _output_get (delegate `FliterChanged`)))

(event `FliterChanged`
  (bind _staticmesh (`self.StaticMesh`))
  (switch `/Game/Elements/Blueprint/E_Filters` (`/Game/VRTemplate/Blueprints/VRGameMode.CurrentFilter` (`self.VRGameModeRef`))
    (:`NewEnumerator0`
      (`PrimitiveComponent.SetMaterial` _staticmesh 0 "/Game/Elements/3D/M_TestFilterNone.M_TestFilterNone"))
    (:`NewEnumerator1`
      (`PrimitiveComponent.SetMaterial` _staticmesh 0 "/Game/Elements/3D/M_TestFilterRed.M_TestFilterRed"))
    (:`NewEnumerator2`
      (`PrimitiveComponent.SetMaterial` _staticmesh 0 "/Game/Elements/3D/M_TestFilterGreen.M_TestFilterGreen"))
    (:`NewEnumerator3`
      (`PrimitiveComponent.SetMaterial` _staticmesh 0 "/Game/Elements/3D/M_TestFilterBlue.M_TestFilterBlue"))))

(fn `UserConstructionScript`)