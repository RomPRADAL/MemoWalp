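; BP_AppearFilter is a 3D element that appears and blocks only while the game mode's current color filter matches its FilterToAppear.
; On BeginPlay it applies the configured static mesh and binds to the VRGameMode filter-changed event.
; Each change swaps the mesh material for the active filter, then toggles mesh visibility and the linked blocking volume's collision on a match.
; It does not evaluate the filter at startup, only when that event fires.
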(event `FliterChanged`
  (bind _staticmesh (`self.StaticMesh`))
  (bind _currentfilter (`/Game/VRTemplate/Blueprints/VRGameMode.CurrentFilter` (`self.VRGameModeRef`)))
  (switch `/Game/Elements/Blueprint/E_Filters` _currentfilter
    (:`NewEnumerator0`
      (`PrimitiveComponent.SetMaterial` _staticmesh 0 "/Game/Elements/3D/M_TestFilterNone.M_TestFilterNone"))
    (:`NewEnumerator1`
      (`PrimitiveComponent.SetMaterial` _staticmesh 0 "/Game/Elements/3D/M_TestFilterRed.M_TestFilterRed"))
    (:`NewEnumerator2`
      (`PrimitiveComponent.SetMaterial` _staticmesh 0 "/Game/Elements/3D/M_TestFilterGreen.M_TestFilterGreen"))
    (:`NewEnumerator3`
      (`PrimitiveComponent.SetMaterial` _staticmesh 0 "/Game/Elements/3D/M_TestFilterBlue.M_TestFilterBlue")))
  (if (`|EnumEquality` _currentfilter (`self.FilterToAppear`))
    (`SceneComponent.SetVisibility` (`self.StaticMesh`) true false)
    (`SceneComponent.SetHiddenInGame` (`self.DefaultSceneRoot`) false false)
    (`PrimitiveComponent.SetCollisionEnabled` (`Brush.BrushComponent` (`self.LinkedBlockingVolume`)) "QueryAndPhysics")
    (else
      (`SceneComponent.SetVisibility` (`self.StaticMesh`) false false)
      (`SceneComponent.SetHiddenInGame` (`self.DefaultSceneRoot`) false false)
      (`PrimitiveComponent.SetCollisionEnabled` (`Brush.BrushComponent` (`self.LinkedBlockingVolume`)) "NoCollision"))))

(event `self.ReceiveBeginPlay`
  (`StaticMeshComponent.SetStaticMesh` (`self.StaticMesh`) (`self.StaticMeshToSet`))
  (bind _asvrgame_mode (cast `/Game/VRTemplate/Blueprints/VRGameMode` (`GameplayStatics.GetGameMode`)))
  (bind _output_get (set `self.VRGameModeRef` _asvrgame_mode))
  (add `/Game/VRTemplate/Blueprints/VRGameMode.FilterChanged` _output_get (delegate `FliterChanged`)))

(fn `UserConstructionScript`)