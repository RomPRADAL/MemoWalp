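; BP_Door is a labyrinth door that is removed once the square, cylinder and pyramid shape boxes have all reported their shape in.
; On BeginPlay it binds to shape-in and win-check events on the three referenced boxes.
; Each shape-in increments a counter, prints it and teleports that box far off-world instead of destroying it.
; The shared win check destroys the door once the counter reaches three.
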(event `self.ReceiveBeginPlay`
  (add `/Game/Elements/3D/Labyrinth/BP_BoxSquare.ShapeIn` (`self.BP_BoxSquare`) (delegate `SquareIn`))
  (add `/Game/Elements/3D/Labyrinth/BP_BoxCylindre.ShapeIn` (`self.BP_BoxCylindre`) (delegate `CylindreIn`))
  (add `/Game/Elements/3D/Labyrinth/Bp_BoxPyramide.ShapeIn` (`self.BP_BoxPyramide`) (delegate `PyramideIn`))
  (add `/Game/Elements/3D/Labyrinth/BP_BoxSquare.WinCheckSquare` (`self.BP_BoxSquare`) (delegate `WinCheck`))
  (add `/Game/Elements/3D/Labyrinth/BP_BoxCylindre.WinCheckCylin` (`self.BP_BoxCylindre`) (delegate `WinCheck`))
  (add `/Game/Elements/3D/Labyrinth/Bp_BoxPyramide.WinCheckPyram` (`self.BP_BoxPyramide`) (delegate `WinCheck`)))

(event `SquareIn`
  (bind _output_get (set `self.DoorOpener` (+ (`self.DoorOpener`) 1)))
  (`KismetSystemLibrary.PrintString` (`KismetStringLibrary.Conv_IntToString` _output_get))
  (`SceneComponent.K2_SetWorldLocation` (`Actor.RootComponent` (`self.BP_BoxSquare`)) (100000000.0 0.0 0.0) false false))

(event `CylindreIn`
  (bind _output_get (set `self.DoorOpener` (+ (`self.DoorOpener`) 1)))
  (`KismetSystemLibrary.PrintString` (`KismetStringLibrary.Conv_IntToString` _output_get))
  (`SceneComponent.K2_SetWorldLocation` (`Actor.RootComponent` (`self.BP_BoxCylindre`)) (1000000000.0 0.0 0.0) false false))

(event `PyramideIn`
  (bind _output_get (set `self.DoorOpener` (+ (`self.DoorOpener`) 1)))
  (`KismetSystemLibrary.PrintString` (`KismetStringLibrary.Conv_IntToString` _output_get))
  (`SceneComponent.K2_SetWorldLocation` (`Actor.RootComponent` (`self.BP_BoxPyramide`)) (100000000.0 0.0 0.0) false false))

(event `WinCheck`
  (`KismetSystemLibrary.PrintString` "Win check activated")
  (if (>= (`self.DoorOpener`) 3)
    (`self.K2_DestroyActor`)))

(fn `UserConstructionScript`)