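; Labyrinth box that detects when a grabbable BP_Pyramide is dropped inside it, apparently as a shape-sorting target.
; Box overlap with the pyramid binds to its GrabComponent's OnDropped event and flags the collision.
; A drop while flagged calls the ShapeIn and WinCheckPyram dispatchers, then clears the flag.
; Ending overlap with a pyramid clears the flag and calls ShapeOut.
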(event `self.Box.OnComponentBeginOverlap`
  (params (OverlappedComponent :type "PrimitiveComponent Object Reference") (OtherActor :type "Actor Object Reference") (OtherComp :type "PrimitiveComponent Object Reference") (OtherBodyIndex :type Integer) (bFromSweep :type Boolean) (SweepResult :type "HitResult Structure (by ref)"))
  (bind _asbp_pyramide (cast `/Game/Elements/3D/Labyrinth/BP_Pyramide` OtherActor))
  (bind _output_get (set `self.GrabRef` (`/Game/Elements/3D/Labyrinth/BP_Pyramide.GrabComponent` _asbp_pyramide)))
  (add `/Game/VRTemplate/Blueprints/GrabComponent.OnDropped` _output_get (delegate `Do`))
  (set `self.IsCollisioned` true))

(event `Do`
  (if (`self.IsCollisioned`)
    (`self.ShapeIn`)
    (`self.WinCheckPyram`)
    (set `self.IsCollisioned` false)))

(event `self.Box.OnComponentEndOverlap`
  (params (OverlappedComponent :type "PrimitiveComponent Object Reference") (OtherActor :type "Actor Object Reference") (OtherComp :type "PrimitiveComponent Object Reference") (OtherBodyIndex :type Integer))
  (cast `/Game/Elements/3D/Labyrinth/BP_Pyramide` OtherActor)
  (set `self.IsCollisioned` false)
  (`self.ShapeOut`))

(fn `Shape In`)

(fn `UserConstructionScript`)