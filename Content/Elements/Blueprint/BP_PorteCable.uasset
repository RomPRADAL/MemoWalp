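; BP_PorteCable is a puzzle door that opens once three referenced cables are all linked.
; On BeginPlay it binds OpenDoor to each cable's FinEnigmeCable event, so every notification rechecks all three IsLinked flags.
; When all pass, it snaps the door to a fixed world rotation and disables collision on its linked blocking volume.
; No closing logic is wired; a collision re-enable node is left disconnected.
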(event `self.ReceiveBeginPlay`
  (add `/Game/Elements/Blueprint/BP_câble.FinEnigmeCable` (`self.BP_CableRef`) (delegate `OpenDoor`))
  (add `/Game/Elements/Blueprint/BP_câble.FinEnigmeCable` (`self.BP_CableRef2`) (delegate `OpenDoor`))
  (add `/Game/Elements/Blueprint/BP_câble.FinEnigmeCable` (`self.BP_CableRef3`) (delegate `OpenDoor`)))

(event `OpenDoor`
  (if (`/Game/Elements/Blueprint/BP_câble.IsLinked` (`self.BP_CableRef`))
    (if (`/Game/Elements/Blueprint/BP_câble.IsLinked` (`self.BP_CableRef2`))
      (if (`/Game/Elements/Blueprint/BP_câble.IsLinked` (`self.BP_CableRef3`))
        (`SceneComponent.K2_SetWorldRotation` (`self.Door`) (struct :`Yaw` 90.0) false false)
        (`PrimitiveComponent.SetCollisionEnabled` (`Brush.BrushComponent` (`self.LinkedBlockingVolume`)) "NoCollision")))))

(fn `UserConstructionScript`)