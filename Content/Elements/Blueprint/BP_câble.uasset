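; BP_câble is a VR cable actor with a grabbable ball end and a rigged cylinder whose material reacts to the active filter.
; On the game mode's filter change, the cylinder shows its filter material if CableFilter matches, otherwise the no-filter material.
; Dropping reapplies the ball's starting world transform as a relative transform.
; Sphere overlap with a BP_Prise socket only prints debug success, without attaching anything.
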(event `self.ReceiveBeginPlay`
  (set `self.PositionDepart` (`SceneComponent.K2_GetComponentToWorld` (`self.LaBoule`)))
  (bind _asvrgame_mode (cast `/Game/VRTemplate/Blueprints/VRGameMode` (`GameplayStatics.GetGameMode`)))
  (bind _output_get (set `self.VRGameModeRef` _asvrgame_mode))
  (add `/Game/VRTemplate/Blueprints/VRGameMode.FilterChanged` _output_get (delegate `FliterChanged`)))

(event `FliterChanged`
  (if (`|EnumEquality` (`/Game/VRTemplate/Blueprints/VRGameMode.CurrentFilter` (`self.VRGameModeRef`)) (`self.CableFilter`))
    (`PrimitiveComponent.SetMaterial` (`self.Rigged_Cylinder`) 0 (`self.MaterialFilter`))
    (else
      (`PrimitiveComponent.SetMaterial` (`self.Rigged_Cylinder`) 0 "/Game/Elements/3D/M_TestFilterNone.M_TestFilterNone"))))

(event `self.GrabComponent.OnDropped`
  (`SceneComponent.K2_SetRelativeTransform` (`self.LaBoule`) (`self.PositionDepart`) false false))

(event `self.Sphèrecollision.OnComponentBeginOverlap`
  (params (OverlappedComponent :type "PrimitiveComponent Object Reference") (OtherActor :type "Actor Object Reference") (OtherComp :type "PrimitiveComponent Object Reference") (OtherBodyIndex :type Integer) (bFromSweep :type Boolean) (SweepResult :type "HitResult Structure (by ref)"))
  (`KismetSystemLibrary.PrintString` (`KismetSystemLibrary.GetObjectName` OtherComp))
  (bind _asbp_prise (cast `/Game/Elements/Blueprint/BP_Prise` OtherActor))
  (`KismetSystemLibrary.PrintString` "Bravo, le cable est bien attaché!"))

(fn `UserConstructionScript`)