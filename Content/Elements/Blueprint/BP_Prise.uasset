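; BP_Prise is an element actor whose cube changes material to match the active filter in the VR game mode.
; On BeginPlay it casts the game mode to VRGameMode and binds to its filter-changed notification.
; When notified, it compares the current filter to its own PriseFIlter, applying MaterialFilter on a match and M_TestFilterNone otherwise.
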(event `self.ReceiveBeginPlay`
  (bind _asvrgame_mode (cast `/Game/VRTemplate/Blueprints/VRGameMode` (`GameplayStatics.GetGameMode`)))
  (bind _output_get (set `self.As VRGame Mode` _asvrgame_mode))
  (add `/Game/VRTemplate/Blueprints/VRGameMode.FilterChanged` _output_get (delegate `FliterChanged`)))

(event `FliterChanged`
  (if (`|EnumEquality` (`/Game/VRTemplate/Blueprints/VRGameMode.CurrentFilter` (`self.As VRGame Mode`)) (`self.PriseFIlter`))
    (`PrimitiveComponent.SetMaterial` (`self.Cube`) 0 (`self.MaterialFilter`))
    (else
      (`PrimitiveComponent.SetMaterial` (`self.Cube`) 0 "/Game/Elements/3D/M_TestFilterNone.M_TestFilterNone"))))

(fn `UserConstructionScript`)